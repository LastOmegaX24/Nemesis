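; CrystalEntity is a destructible crystal actor that explodes when it takes any positive damage.
; The AnyDamage event re-emits the received amount as radial damage with falloff within Radius, crediting the original instigator and ignoring the original damage causer.
; It then spawns the CrystalExplosion effect at its location and destroys itself.
; An ApplyDamage call on itself is left unconnected.
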(event `self.ReceiveBeginPlay`)

(event `self.ReceiveAnyDamage`
  (params (Damage :type "Float (single-precision)") (DamageType :type "DamageType Object Reference") (InstigatedBy :type "Controller Object Reference") (DamageCauser :type "Actor Object Reference"))
  (bind _returnvalue (`self.K2_GetActorLocation`))
  (if (> Damage 0.0)
    (`GameplayStatics.ApplyRadialDamageWithFalloff` (`self.Damage`) 0.0 _returnvalue 0.0 (`self.Radius`) 0.0 null (`|MakeArray` DamageCauser) self InstigatedBy)
    (`NiagaraFunctionLibrary.SpawnSystemAtLocation` "/Game/Nemesis/Particle/CrystalExplosion.CrystalExplosion" _returnvalue)
    (`self.K2_DestroyActor`)))

(fn `UserConstructionScript`)