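; Sword actor Blueprint that attaches its skeletal mesh to a character's left arm when it spawns.
; On BeginPlay it calls the parent logic, then plays the non-looping SheathPowering animation on the mesh.
; If the Character reference is valid, the mesh snaps to the arm_L_001 socket location, keeping world rotation and scale.
; Overlap and Tick events are disabled, and the construction script only calls its parent.
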(event `self.ReceiveBeginPlay`
  (`parent.ReceiveBeginPlay`)
  (`SkeletalMeshComponent.PlayAnimation` (`self.SkeletalMesh1`) "/Game/Nemesis/Assets/Other/SheathPowering.SheathPowering" false)
  (bind _character (`self.Character`)
    (:`then`
      (`SceneComponent.K2_AttachToComponent` (`self.SkeletalMesh1`) (`Character.Mesh` _character) "arm_L_001" "SnapToTarget" "KeepWorld" "KeepWorld" true))
    (:`else`)))

(fn `UserConstructionScript`
  (`parent.UserConstructionScript`))