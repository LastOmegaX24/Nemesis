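; Sword weapon Blueprint that detects melee hits and applies damage and knockback.
; Attack stores the attack index and restarts a sphere MeleeTrace between the hit_start and hit_end sockets; EndAttack stops it.
; Trace hits on actors other than the owner apply damage scaled by a global and per-attack multiplier.
; Each hit also messages the victim with per-attack knockback, oriented from the owner toward the victim.
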(event `self.Attack`
  (params (AtkIndex :type Integer))
  (bind _traceinfo (`self.TraceInfo`))
  (set `self.AtkIndex` AtkIndex)
  (if (`MeleeTraceComponent.IsMeleeTraceHandleValid` _traceinfo)
    (`MeleeTraceComponent.EndTrace` (`self.MeleeTrace`) _traceinfo))
  (bind _returnvalue (`MeleeTraceComponent.StartTrace` (`self.MeleeTrace`) (make `MeleeTraceInfo` "hit_start" "hit_end" (`MeleeTraceShape_Sphere.MakeSphereShape` 3.0) 3)))
  (set `self.TraceInfo` _returnvalue))

(event `self.EndAttack`
  (`MeleeTraceComponent.EndTrace` (`self.MeleeTrace`) (`self.TraceInfo`)))

(event `self.MeleeTrace.OnTraceHit`
  (params (ThisComponent :type "MeleeTraceComponent Object Reference") (HitActor :type "Actor Object Reference") (HitLocation :type "Vector Structure (by ref)") (HitNormal :type "Vector Structure (by ref)") (HitBoneName :type Name) (TraceHandle :type "MeleeTraceInstanceHandle Structure"))
  (bind (_dmg_multiplier _kb_multiplier _dir_knockback) (break `/Game/Nemesis/Blueprints/DMG_Multiplier` (`|GetArrayItem` (`self.DamageMulti`) (`self.AtkIndex`))))
  (if (!= HitActor (`self.GetOwner`))
    (`GameplayStatics.ApplyDamage` HitActor (* (`self.BaseDamage`) (`self.DamageMultiplier`) (`.DMG_Multiplier_8_2A3D00184F934C2AE62A15A3B8A22F4D` (break `/Game/Nemesis/Blueprints/DMG_Multiplier` (`|GetArrayItem` (`self.DamageMulti`) (`self.AtkIndex`))))) (`self.GetInstigatorController`) (`self.GetOwner`) "/Script/Engine.DamageType")
    (message `/Game/Nemesis/Blueprints/Interface/Knockback.DealKnockback` HitActor (`KismetMathLibrary.FindLookAtRotation` (`self.K2_GetActorLocation` (`self.GetOwner`)) (`self.K2_GetActorLocation` HitActor)) _dir_knockback _kb_multiplier)))

(fn `UserConstructionScript`
  (`parent.UserConstructionScript`))