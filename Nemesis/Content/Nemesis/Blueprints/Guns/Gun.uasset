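; Gun weapon Blueprint that supplies third-person shooting animations for characters.
; BeginPlay picks hip and ADS montages by weapon type: light for Sword, heavy for Scythe and Polearm.
; RPCAnimation plays one on the character's mesh through PlayArmAnim based on its ADS flag; as wired, a true flag selects the hip montage.
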(event `self.ReceiveBeginPlay`
  (switch `/Game/Nemesis/Blueprints/WeaponType` (`self.WeaponType`)
    (:`NewEnumerator0`
      (set `self.HIP_Anim` "/Game/Nemesis/ActionAnim/TP/TP_ShootLight.TP_ShootLight")
      (set `self.ADS_Anim` "/Game/Nemesis/ActionAnim/TP/TP_ShootLightADS.TP_ShootLightADS"))
    (:`NewEnumerator1`
      (set `self.HIP_Anim` "/Game/Nemesis/ActionAnim/TP/TP_ShootHeavy.TP_ShootHeavy")
      (set `self.ADS_Anim` "/Game/Nemesis/ActionAnim/TP/TP_ShootHeavyADS.TP_ShootHeavyADS"))
    (:`NewEnumerator2`
      (set `self.HIP_Anim` "/Game/Nemesis/ActionAnim/TP/TP_ShootHeavy.TP_ShootHeavy")
      (set `self.ADS_Anim` "/Game/Nemesis/ActionAnim/TP/TP_ShootHeavyADS.TP_ShootHeavyADS"))))

(event `self.RPC_Animation`
  (params (Character :type "/Game/Nemesis/Old/NS_Character Object Reference"))
  (`self.PlayArmAnim` (select `bool` (`/Game/Nemesis/Old/NS_Character.ADS` Character) :`false` (`self.ADS_Anim`) :`true` (`self.HIP_Anim`)) (`Character.Mesh` Character)))

(fn `UserConstructionScript`)